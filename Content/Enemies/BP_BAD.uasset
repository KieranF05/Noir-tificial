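; BP_BAD is a damageable enemy that can drop a weapon when killed.
; AnyDamage lowers HEALTH and prints debug text; at zero or below, a random integer picks the death outcome.
; One case spawns a Remington 870 and destroys the actor, another does so with no spawn class set, and other rolls leave it alive.
; A TommyGun drop is present but unconnected.
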(event `self.ReceiveAnyDamage`
  (params (Damage :type "Float (single-precision)") (DamageType :type "DamageType Object Reference") (InstigatedBy :type "Controller Object Reference") (DamageCauser :type "Actor Object Reference"))
  (`KismetSystemLibrary.PrintText` "pricko")
  (set `self.HEALTH` (- (`self.HEALTH`) Damage))
  (if (<= (`self.HEALTH`) 0.0)
    (`KismetSystemLibrary.PrintText` "HOLY FUCKT HAT HURT FUCK YOU AWWWWWWWW")
    (switch `int` (`KismetMathLibrary.RandomIntegerInRange` 0 3)
      (:`0`
        (`|SpawnActorFromClass` null (`KismetMathLibrary.MakeTransform` (`self.K2_GetActorLocation`)) "AlwaysSpawn" "MultiplyWithRoot" null null)
        (`self.K2_DestroyActor`))
      (:`2`
        (`|SpawnActorFromClass` "/Game/Models/Weapons/BP_Remington_870.BP_Remington_870_C" (`KismetMathLibrary.MakeTransform` (`self.K2_GetActorLocation`)) "AlwaysSpawn" "MultiplyWithRoot" null null)
        (`self.K2_DestroyActor`)))))

(fn `UserConstructionScript`)